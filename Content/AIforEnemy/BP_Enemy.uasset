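; BP_Enemy is an enemy actor with a health value and a text render that displays it.
; The construction script writes HealtPoint to the text, which is not updated when damage arrives.
; AnyDamage sets HealtPoint to Damage minus HealtPoint (operands reversed from a usual health subtraction) and destroys the actor when the result is zero or below.
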(event `self.ReceiveAnyDamage`
  (params (Damage :type "Float (single-precision)") (DamageType :type "DamageType Object Reference") (InstigatedBy :type "Controller Object Reference") (DamageCauser :type "Actor Object Reference"))
  (bind _output_get (set `self.HealtPoint` (- Damage (`self.HealtPoint`))))
  (if (<= _output_get 0.0)
    (`self.K2_DestroyActor`)))

(fn `UserConstructionScript`
  (`TextRenderComponent.K2_SetText` (`self.TextRender`) (`KismetTextLibrary.Conv_DoubleToText` (`self.HealtPoint`) "HalfToEven")))